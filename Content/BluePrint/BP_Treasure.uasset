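; BP_Treasure is a treasure chest that opens when BP_ThirdPersonCharacter enters its Box trigger and closes when the character leaves.
; On entry, a timeline pitches the Top lid open and restarts a second timeline on each update, so the Book effectively rises afterward and reveals the prompt text.
; On exit, the prompt hides while two separate timelines close the lid and lower the book together.
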(event OnComponentEndOverlap(Box)
  (params (OverlappedComponent :type Primitive%20Component%20Object%20Reference) (OtherActor :type Actor%20Object%20Reference) (OtherComp :type Primitive%20Component%20Object%20Reference) (OtherBodyIndex :type Integer))
  (Utilities|Casting|CastToBP_ThirdPersonCharacter OtherActor)
  (Rendering|SetVisibility (Variables|Default|Get提示文本) false false)
  (Utilities|FlowControl|Sequence
    (:then_0
      (bind _新建轨道_0 (Timeline|时间轴_1 PlayFromStart)
        (:Update
          (Transformation|SetRelativeRotation (Variables|Default|Gettop) (Math|Rotator|MakeRotator 0.0 (Math|Float|Lerp 9e+01 0.0 _新建轨道_0) 0.0) false false))))
    (:then_1
      (bind _新建轨道_0_2 (Timeline|时间轴_2 PlayFromStart)
        (:Update
          (Transformation|SetRelativeLocation (Variables|Default|GetBook) (Math|Vector|MakeVector 0.0 0.0 (Math|Float|Lerp 7e+01 0.0 _新建轨道_0_2)) false false))))))

(event OnComponentBeginOverlap(Box)
  (params (OverlappedComponent :type Primitive%20Component%20Object%20Reference) (OtherActor :type Actor%20Object%20Reference) (OtherComp :type Primitive%20Component%20Object%20Reference) (OtherBodyIndex :type Integer) (bFromSweep :type Boolean) (SweepResult :type Hit%20Result%20Structure%20%28by%20ref%29))
  (Utilities|Casting|CastToBP_ThirdPersonCharacter OtherActor)
  (bind _新建轨道_0 (Timeline|时间轴 PlayFromStart)
    (:Update
      (Transformation|SetRelativeRotation (Variables|Default|Gettop) (Math|Rotator|MakeRotator 0.0 (Math|Float|Lerp 0.0 9e+01 _新建轨道_0) 0.0) false false)
      (bind _新建轨道_0_2 (Timeline|时间轴_0 PlayFromStart)
        (:Update
          (Transformation|SetRelativeLocation (Variables|Default|GetBook) (Math|Vector|MakeVector 0.0 0.0 (Math|Float|Lerp 0.0 7e+01 _新建轨道_0_2)) false false)
          (Rendering|SetVisibility (Variables|Default|Get提示文本) true false))))))

(event EventBeginPlay)

(event Collision|EventActorBeginOverlap
  (params (OtherActor :type Actor%20Object%20Reference)))

(event EventTick
  (params (DeltaSeconds :type Float%20%28single-precision%29)))

(fn ConstructionScript)