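; Treasure chest actor that reveals a book and lets the player travel to the Asian_Village_Demo level.
; When a BP_MasterCharacter with Option matching Num overlaps the Box, timelines swing the lid open, raise the book, show a prompt and open a Gate; leaving reverses this.
; JumpLevel input, enabled by any character overlap, passes through that Gate to show the ShowUI3 widget, then loads the level after a delay.
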(event OnComponentEndOverlap(Box)
  (params (OverlappedComponent :type Primitive%20Component%20Object%20Reference) (OtherActor :type Actor%20Object%20Reference) (OtherComp :type Primitive%20Component%20Object%20Reference) (OtherBodyIndex :type Integer))
  ;[1 1 1] 宝箱关闭
  (bind _asbp_master_character (Utilities|Casting|CastToBP_MasterCharacter OtherActor))
  (if (== (Variables|/Game/ClimbingComponent/Blueprints/CharacterBP/BP_MasterCharacter.BP_MasterCharacter_C|GetOption _asbp_master_character) (Variables|Default|GetNum))
    (Rendering|SetVisibility (Variables|Default|Get提示文本) false false)
    (Utilities|FlowControl|Sequence
      (:then_0
        (bind _新建轨道_0 (Timeline|时间轴_1 PlayFromStart)
          (:Update
            (Transformation|SetRelativeRotation (Variables|Default|Gettop) (Math|Rotator|MakeRotator 0.0 (Math|Float|Lerp 9e+01 0.0 _新建轨道_0) 0.0) false false)
            ;[1 1 1] 宝箱打开
            (Utilities|FlowControl|Gate true) ; enters at Close
          )))
      (:then_1
        (bind _新建轨道_0_2 (Timeline|时间轴_2 PlayFromStart)
          (:Update
            (Transformation|SetRelativeLocation (Variables|Default|GetBook) (Math|Vector|MakeVector 0.0 0.0 (Math|Float|Lerp 7e+01 0.0 _新建轨道_0_2)) false false)))))))

(event OnComponentBeginOverlap(Box)
  (params (OverlappedComponent :type Primitive%20Component%20Object%20Reference) (OtherActor :type Actor%20Object%20Reference) (OtherComp :type Primitive%20Component%20Object%20Reference) (OtherBodyIndex :type Integer) (bFromSweep :type Boolean) (SweepResult :type Hit%20Result%20Structure%20%28by%20ref%29))
  ;[1 1 1] 宝箱打开
  (bind _asbp_master_character (Utilities|Casting|CastToBP_MasterCharacter OtherActor))
  (Input|EnableInput (Game|GetPlayerController 0))
  (Variables|Default|SetCanGet true)
  (if (== (Variables|/Game/ClimbingComponent/Blueprints/CharacterBP/BP_MasterCharacter.BP_MasterCharacter_C|GetOption _asbp_master_character) (Variables|Default|GetNum))
    (bind _新建轨道_0 (Timeline|时间轴 PlayFromStart)
      (:Update
        (Transformation|SetRelativeRotation (Variables|Default|Gettop) (Math|Rotator|MakeRotator 0.0 (Math|Float|Lerp 0.0 9e+01 _新建轨道_0) 0.0) false false)
        (bind _新建轨道_0_2 (Timeline|时间轴_0 PlayFromStart)
          (:Update
            (Transformation|SetRelativeLocation (Variables|Default|GetBook) (Math|Vector|MakeVector 0.0 0.0 (Math|Float|Lerp 0.0 7e+01 _新建轨道_0_2)) false false)
            (Rendering|SetVisibility (Variables|Default|Get提示文本) true false)
            (Utilities|FlowControl|Gate true) ; enters at Open
          ))))))

(event EventBeginPlay)

(event Collision|EventActorBeginOverlap
  (params (OtherActor :type Actor%20Object%20Reference)))

(event EventTick
  (params (DeltaSeconds :type Float%20%28single-precision%29)))

(event Input|ActionEvents|InputActionJumpLevel
  (params (Key :type Key%20Structure :default "None"))
  ;[1 1 1] 宝箱打开
  (:Pressed
    (if (Variables|Default|GetCanGet)
      (Utilities|FlowControl|Gate true
        (:Exit
          (Variables|Default|SetCanGet false)
          (bind _returnvalue (UserInterface|CreateWidget "/Game/BluePrint/ShowUI3.ShowUI3_C"))
          (UserInterface|Viewport|AddtoViewport _returnvalue 0)
          (Utilities|FlowControl|Delay 3.0)
          (Game|OpenLevel(byObjectReference) "/Game/Asian_Village/maps/Asian_Village_Demo.Asian_Village_Demo")))
      (else
        (Development|PrintString "GUN!!!")))))

(fn ConstructionScript)