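; BP_Light is an interactable light that triggers the game's ending.
; Its sphere overlap enables input and shows prompt text while the player is inside.
; Pressing EndGame checks four Renwu quest flags in MyInstance, printing a warning if any is unset.
; Otherwise it toggles the light, plays sound, sequence and timed ending widgets, then opens StartGame; ISOn reports light visibility.
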(event OnComponentBeginOverlap(Sphere)
  (params (OverlappedComponent :type Primitive%20Component%20Object%20Reference) (OtherActor :type Actor%20Object%20Reference) (OtherComp :type Primitive%20Component%20Object%20Reference) (OtherBodyIndex :type Integer) (bFromSweep :type Boolean) (SweepResult :type Hit%20Result%20Structure%20%28by%20ref%29))
  (bind _asbp_third_person_character (Utilities|Casting|CastToBP_ThirdPersonCharacter OtherActor))
  (Input|EnableInput (.As玩家控制器 (Utilities|Casting|CastToPlayerController (Pawn|GetController _asbp_third_person_character))))
  (Rendering|SetVisibility (Variables|Default|Get提示文本) true false))

(event OnComponentEndOverlap(Sphere)
  (params (OverlappedComponent :type Primitive%20Component%20Object%20Reference) (OtherActor :type Actor%20Object%20Reference) (OtherComp :type Primitive%20Component%20Object%20Reference) (OtherBodyIndex :type Integer))
  (bind _asbp_third_person_character (Utilities|Casting|CastToBP_ThirdPersonCharacter OtherActor))
  (Input|DisableInput (.As玩家控制器 (Utilities|Casting|CastToPlayerController (Pawn|GetController _asbp_third_person_character))))
  (Rendering|SetVisibility (Variables|Default|Get提示文本) false false))

(event EventBeginPlay)

(event Collision|EventActorBeginOverlap
  (params (OtherActor :type Actor%20Object%20Reference)))

(event EventTick
  (params (DeltaSeconds :type Float%20%28single-precision%29)))

(event Input|ActionEvents|InputActionEndGame
  (params (Key :type Key%20Structure :default "None"))
  (:Pressed
    (bind _asmy_instance (Utilities|Casting|CastToMyInstance (Game|GetGameInstance)))
    (if (Math|Boolean|ANDBoolean (Variables|/Game/MyInstance/MyInstance.MyInstance_C|Getrenwu1 _asmy_instance) (Variables|/Game/MyInstance/MyInstance.MyInstance_C|Getrenwu2 _asmy_instance) (Variables|/Game/MyInstance/MyInstance.MyInstance_C|Getrenwu3 _asmy_instance) (Variables|/Game/MyInstance/MyInstance.MyInstance_C|Getrenwu4 _asmy_instance))
      (Rendering|ToggleVisibility (Variables|Default|GetPointLight) false)
      (Utilities|FlowControl|Delay 1.0)
      (Audio|PlaySound2D "/Game/Movies/Vedio/EndGame.EndGame" 1.0 1.0 0.0 0 0)
      (Input|DisableInput (Game|GetPlayerCharacter 0) (Game|GetPlayerController 0))
      (bind (_outactor _returnvalue) (Sequencer|Player|CreateLevelSequencePlayer "/Game/Kobo_Nature/LevelSequence/MainLevelSequence.MainLevelSequence"))
      (Sequencer|Player|Play (Variables|/Script/LevelSequence.LevelSequenceActor|GetSequencePlayer _outactor) :!class /Script/MovieScene.MovieSceneSequencePlayer)
      (bind _returnvalue_2 (UserInterface|CreateWidget "/Game/Asian_Village/UI/END01.END01_C"))
      (UserInterface|Viewport|AddtoViewport _returnvalue_2 0)
      (Rendering|SetVisibility (Variables|Default|Get提示文本) false false)
      (Utilities|FlowControl|Delay 42.0)
      (Widget|SetVisibility (Variables|/Game/Asian_Village/UI/END01.END01_C|GetCanvasPanel_19 _returnvalue_2) "Collapsed")
      (bind _returnvalue_3 (UserInterface|CreateWidget "/Game/Asian_Village/UI/G_E_T.G_E_T_C"))
      (UserInterface|Viewport|AddtoViewport _returnvalue_3 0)
      (UserInterface|Animation|PlayAnimation _returnvalue_3 (Variables|/Game/Asian_Village/UI/G_E_T.G_E_T_C|GetGameEnd _returnvalue_3) 0.0 1 "Forward" 1.0 false)
      (Utilities|FlowControl|Delay 7.0)
      (Game|OpenLevel(byObjectReference) "/Game/Asian_Village/maps/StartGame.StartGame")
      (else
        (Development|PrintString "条件不够，请完成关卡挑战再来！")))))

(fn ConstructionScript)

(fn ISon
  (return (Variables|/Script/Engine.SceneComponent|GetbVisible (Variables|Default|GetPointLight))))