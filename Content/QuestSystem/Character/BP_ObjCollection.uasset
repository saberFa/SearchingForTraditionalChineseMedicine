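; Quest objective collection that groups child objectives and counts as complete only when every child is complete.
; On activation it either activates all children at once or, when order is required, runs them one by one.
; In ordered mode it activates the first incomplete child, then binds to its completion event to unbind and advance to the next.
; The file shows no completion broadcast from the collection itself.
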(event Custom|OnComplated_事件
  (params (Obj :type BP%20Objective%20Object%20Reference) (roo :type My%20Instance%20Object%20Reference))
  (EventDispatchers|UnbindEventfromOnComplated Obj (delegate Custom|OnComplated_事件))
  (bind _nextobj (CallFunction|FindNextincomplateObj))
  (Utilities|IsValid _nextobj
    (:Is%20Valid
      (Default|ActiveObj _nextobj)
      (EventDispatchers|AssignOnComplated _nextobj (delegate Custom|OnComplated_事件)))))

(event EventActiveObj
  (|CallParentFunction)
  (if (Variables|Default|GetOrderRequired)
    (bind _nextobj (CallFunction|FindNextincomplateObj))
    (Utilities|IsValid _nextobj
      (:Is%20Valid
        (Default|ActiveObj _nextobj)
        (EventDispatchers|AssignOnComplated _nextobj (delegate Custom|OnComplated_事件))))
    (else
      (for _array_element (Variables|Default|GetObjs)
        (Default|ActiveObj _array_element)))))

(fn FindNextincomplateObj
  (for _array_element (Variables|Default|GetObjs)
    (if (not (CallFunction|GetIsComplate _array_element))
      (return _array_element)))
  (return 0))

(fn AddObj
  (params (Obj :type BP%20Objective%20Object%20Reference%20%28by%20ref%29))
  (Utilities|Array|Add (Variables|Default|GetObjs) Obj))

(fn GetIsComplate
  (for _array_element (Variables|Default|GetObjs)
    (if (not (CallFunction|GetIsComplate _array_element))
      (return false)))
  (return true))