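; Quest objective that completes when the player character reaches a Destination actor.
; On activation it binds to that actor's begin-overlap event, then unbinds on the first BP_ThirdPersonCharacter overlap and marks itself complete.
; It also sets the first unset of four sequential Renwu progress flags, then fires the OnComplated dispatcher with itself and Renwu.
; GetIsComplate reports the objective's own completion flag, Renwu0.
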(event Custom|OnActorBeginOverlap_事件
  (params (OverlappedActor :type Actor%20Object%20Reference) (OtherActor :type Actor%20Object%20Reference))
  (bind _renwu (Variables|Default|Getrenwu))
  (bind _renwu_2 (Variables|Default|Getrenwu))
  (bind _renwu_3 (Variables|Default|Getrenwu))
  (bind _renwu_4 (Variables|Default|Getrenwu))
  (Utilities|Casting|CastToBP_ThirdPersonCharacter OtherActor)
  (Collision|UnbindEventfromOnActorBeginOverlap (Variables|Default|GetDestination) (delegate Custom|OnActorBeginOverlap_事件))
  ;[1 1 1] 保存和设置关卡变量
  (Variables|Default|Setrenwu0 true)
  (if (Variables|/Game/MyInstance/MyInstance.MyInstance_C|Getrenwu1 _renwu)
    (if (Variables|/Game/MyInstance/MyInstance.MyInstance_C|Getrenwu2 _renwu_2)
      (if (Variables|/Game/MyInstance/MyInstance.MyInstance_C|Getrenwu3 _renwu_3)
        (if (Variables|/Game/MyInstance/MyInstance.MyInstance_C|Getrenwu4 _renwu_4)
          (Default|CallOnComplated self _renwu_4)
          (else
            (Variables|/Game/MyInstance/MyInstance.MyInstance_C|Setrenwu4 _renwu_4 true)
            (Default|CallOnComplated self _renwu_4)))
        (else
          (Variables|/Game/MyInstance/MyInstance.MyInstance_C|Setrenwu3 _renwu_3 true)
          (Default|CallOnComplated self _renwu_3)))
      (else
        (Variables|/Game/MyInstance/MyInstance.MyInstance_C|Setrenwu2 _renwu_2 true)
        (Default|CallOnComplated self _renwu_2)))
    (else
      (Variables|/Game/MyInstance/MyInstance.MyInstance_C|Setrenwu1 _renwu true)
      (Default|CallOnComplated self _renwu))))

(event EventActiveObj
  (|CallParentFunction)
  (EventDispatchers|AssignOnActorBeginOverlap (Variables|Default|GetDestination) (delegate Custom|OnActorBeginOverlap_事件)))

(fn GetIsComplate
  (return (Variables|Default|Getrenwu0)))