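; BP_Q_1 is a side quest (支线任务) with four objectives, the keys of 望, 闻, 问 and 切.
; It builds an unordered root BP_ObjCollection and fills it with BP_ObjReachDestination objectives, each tied to its own destination reference.
; Each objective also receives the RenWu object from the parent's GetRenWu and that object's matching numbered Renwu field.
; A separate helper returns the game instance cast to MyInstance.
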(fn ConstructionScript
  (|CallParentFunction))

(fn ConstructRootObjCollection
  (bind _returnvalue (Game|ConstructObjectfromClass self "/Game/QuestSystem/Character/BP_ObjCollection.BP_ObjCollection_C" false "支线任务"))
  (return _returnvalue))

(fn PopulateObj
  (params (RootObjCollection :type BP%20Obj%20Collection%20Object%20Reference))
  (Utilities|FlowControl|Sequence
    (:then_0
      ;[1 1 1] 闯将任务面板
      (bind _newparam (CallFunction|GetRenWu))
      (bind _returnvalue (Game|ConstructObjectfromClass "/Game/QuestSystem/Character/BP_ObjReachDestination.BP_ObjReachDestination_C" (Variables|Default|GetMegatonTrigger) _newparam (Variables|/Game/MyInstance/MyInstance.MyInstance_C|Getrenwu1 _newparam) "任务之一：”望“之钥"))
      (Default|AddObj RootObjCollection _returnvalue))
    (:then_1
      (bind _newparam_2 (CallFunction|GetRenWu))
      (bind _returnvalue_2 (Game|ConstructObjectfromClass "/Game/QuestSystem/Character/BP_ObjReachDestination.BP_ObjReachDestination_C" (Variables|Default|GetMegatonTrigger1) _newparam_2 (Variables|/Game/MyInstance/MyInstance.MyInstance_C|Getrenwu2 _newparam_2) "任务之二：”闻“之钥"))
      (Default|AddObj RootObjCollection _returnvalue_2))
    (:then_2
      (bind _newparam_3 (CallFunction|GetRenWu))
      (bind _returnvalue_3 (Game|ConstructObjectfromClass "/Game/QuestSystem/Character/BP_ObjReachDestination.BP_ObjReachDestination_C" (Variables|Default|GetSphereTrigger) _newparam_3 (Variables|/Game/MyInstance/MyInstance.MyInstance_C|Getrenwu3 _newparam_3) "任务之三：”问“之钥"))
      (Default|AddObj RootObjCollection _returnvalue_3))
    (:then_3
      (bind _newparam_4 (CallFunction|GetRenWu))
      (bind _returnvalue_4 (Game|ConstructObjectfromClass "/Game/QuestSystem/Character/BP_ObjReachDestination.BP_ObjReachDestination_C" (Variables|Default|Get任务4) _newparam_4 (Variables|/Game/MyInstance/MyInstance.MyInstance_C|Getrenwu4 _newparam_4) "任务之四：”切“之钥"))
      (Default|AddObj RootObjCollection _returnvalue_4))))

(fn Castto
  (bind _returnvalue (Game|GetGameInstance))
  (Utilities|IsValid _returnvalue
    (:Is%20Valid
      (bind _asmy_instance (Utilities|Casting|CastToMyInstance _returnvalue))
      (return _asmy_instance))))

(fn GetRenWu
  (bind _newparam (|CallParentFunction))
  (return _newparam))