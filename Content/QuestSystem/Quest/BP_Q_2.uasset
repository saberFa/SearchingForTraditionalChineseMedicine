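; BP_Q_2 is a quest Blueprint that defines a main quest (主线任务) built from turn-on-light objectives labeled "collect the lost key" (收集失落的钥匙).
; It overrides its parent's construction hooks to create an unordered BP_ObjCollection as the root.
; PopulateObj adds one BP_ObjTurnOnLight per Light array entry, passing each the light and the RenWu reference from the parent getter.
; The event graph holds only disabled or empty stubs.
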(event EventBeginPlay
  (|CallParentFunction) ; 此节点被禁用，将不会被调用。\n从引脚连出引线来编译功能。
)

(event Collision|EventActorBeginOverlap
  (params (OtherActor :type Actor%20Object%20Reference)))

(event EventTick
  (params (DeltaSeconds :type Float%20%28single-precision%29)))

(fn ConstructionScript
  (|CallParentFunction))

(fn ConstructRootObjCollection
  (bind _returnvalue (Game|ConstructObjectfromClass self "/Game/QuestSystem/Character/BP_ObjCollection.BP_ObjCollection_C" false "主线任务"))
  (return _returnvalue))

(fn PopulateObj
  (params (RootObjCollection :type BP%20Obj%20Collection%20Object%20Reference))
  (bind _newparam (CallFunction|GetRenWu))
  (for _array_element (Variables|Default|GetLight)
    (bind _returnvalue (Game|ConstructObjectfromClass "/Game/QuestSystem/Character/BP_ObjTurnOnLight.BP_ObjTurnOnLight_C" _array_element _newparam (Utilities|Text|FormatText "收集失落的钥匙")))
    (Default|AddObj RootObjCollection _returnvalue)))

(fn GetRenWu
  (bind _newparam (|CallParentFunction))
  (return _newparam))