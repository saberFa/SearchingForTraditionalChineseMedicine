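; BP_Q is a base quest Blueprint that builds and activates a collection of quest objectives.
; On BeginPlay it constructs and stores RootObjCollection, populates it through PopulateObj, calls GetRenWu, then calls ActiveObj on the collection.
; ConstructRootObjCollection and PopulateObj are meant for child overrides; the base versions only print red error messages.
; GetRenWu returns the game instance cast to MyInstance, though BeginPlay does not use the result.
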(event EventBeginPlay
  (bind _rootobjcollection (Private|ConstructRootObjCollection))
  (bind _output_get (Variables|Private|SetRootObjCollection _rootobjcollection))
  (Private|PopulateObj _output_get)
  (CallFunction|GetRenWu)
  (Default|ActiveObj (Variables|Private|GetRootObjCollection)))

(fn ConstructionScript)

(fn PopulateObj
  (params (RootObjCollection :type BP%20Obj%20Collection%20Object%20Reference))
  (Development|PrintString "错误：PopulateObj call for base class!" true true "(R=1.000000,G=0.000000,B=0.044590,A=1.000000)"))

(fn ConstructRootObjCollection
  (Development|PrintString "错误：ConstructRootObjCollection call for base class!" true true "(R=1.000000,G=0.009094,B=0.000000,A=1.000000)")
  (return 0))

(fn GetRootObjCollection
  (return (Variables|Private|GetRootObjCollection)))

(fn GetRenWu
  (bind _asmy_instance (Utilities|Casting|CastToMyInstance (Game|GetGameInstance)))
  (return _asmy_instance))