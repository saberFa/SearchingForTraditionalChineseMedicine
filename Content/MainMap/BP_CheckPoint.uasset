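; BP_CheckPoint is a checkpoint marker actor that shows an icon on the main map through a Wjb_mainmap_icon widget, created shortly after BeginPlay.
; It attaches its CalcHelper component to the player character's root.
; Each Tick it moves CalcHelper to the checkpoint's world location and feeds the resulting player-relative XY offset to the widget.
; The icon also sets the editor billboard sprite; no overlap logic is implemented.
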(event EventBeginPlay
  (Utilities|FlowControl|Delay 0.5)
  (bind _returnvalue (UserInterface|CreateWidget "/Game/MainMap/wjb_mainmap_icon.wjb_mainmap_icon_C"))
  (bind _output_get (Variables|Default|Setmainmap_icon _returnvalue))
  (Default|ChangeIcon _output_get (Variables|Default|GetIcon))
  (Default|ChangeSize _output_get (Variables|Default|GetIconSize))
  (UserInterface|Viewport|AddtoViewport _output_get 0)
  (Transformation|AttachComponentToComponent (Variables|Default|Getcalc_helper) (Variables|/Script/Engine.Actor|GetRootComponent (Game|GetPlayerCharacter 0)) "None" "KeepWorld" "KeepWorld" "KeepWorld" false)
  (CallFunction|UpdateIconPosition))

(event Collision|EventActorBeginOverlap
  (params (OtherActor :type Actor%20Object%20Reference)))

(event EventTick
  (params (DeltaSeconds :type Float%20%28single-precision%29))
  (CallFunction|UpdateIconPosition))

(fn ConstructionScript
  (Rendering|Components|Sprite|SetSprite (Variables|Default|GetBillboard) (Variables|Default|GetIcon)))

(fn UpdateIconPosition
  (Transformation|SetWorldLocation (Variables|Default|Getcalc_helper) (Transformation|GetActorLocation) false false)
  (bind _mainmap_icon (Variables|Default|Getmainmap_icon)
    (:then
      (Default|UpdateIocnLocation _mainmap_icon (Math|Conversions|ToVector2D(Vector) (Variables|/Script/Engine.SceneComponent|GetRelativeLocation (Variables|Default|Getcalc_helper)))))
    (:else)))