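; Debug character that repeatedly plays a test montage or animation sequence in place to preview climbing-component animations.
; On BeginPlay it can snap to a desired distance from a wall ahead, then plays in Flying mode, returns to Walking, and resets its transform to loop.
; Sequences become dynamic montages; an optional timer draws debug spheres at the root bone to trace its path when the player is near.
; A helper macro stops a given or active montage after a delay.
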(fn ConstructionScript)

(event Custom|Leave%20Debug%20traces%20for%20Root
  (if (< (Transformation|GetDistanceTo (Game|GetPlayerCharacter 0)) 6e+02)
    (Rendering|Debug|DrawDebugSphere (Transformation|GetWorldLocation (Variables|Default|GetSphere)) 5.0 1 "(R=1.000000,G=0.891186,B=0.000000,A=1.000000)" 2.0 2.0)))

(event EventBeginPlay
  (bind _returnvalue (Transformation|GetActorLocation))
  (bind _alphablendargs (Utilities|Struct|MakeAlphaBlendArgs 0 0.2 "Linear"))
  (bind _animsequence_to_test (Variables|Default|GetAnimSequence%20to%20test))
  (bind _returnvalue_2 (Utilities|IsValid _animsequence_to_test))
  (if (Variables|Default|GetTrace%20Root)
    (Utilities|Time|SetTimerbyEvent (delegate Custom|Leave%20Debug%20traces%20for%20Root) 0.05 true))
  (bind _outhit (Collision|SphereTraceForObjects _returnvalue (+ _returnvalue (* (Transformation|GetActorForwardVector) 2e+02)) 3e+01 (Utilities|Array|MakeArray "ObjectTypeQuery1") false 0 "None"))
  (if (Variables|Default|GetSet%20Desired%20Distance)
    (if (.bBlockingHit (Collision|BreakHitResult _outhit))
      (Transformation|SetActorLocation (+ (.ImpactPoint (Collision|BreakHitResult _outhit)) (* (.ImpactNormal (Collision|BreakHitResult _outhit)) (Variables|Default|GetDesired%20Distance))) false true)))
  (Variables|Default|SetLocation (Transformation|GetActorLocation))
  (Variables|Default|SetRot (Transformation|GetActorRotation))
  (Transformation|AttachComponentToComponent (Variables|Default|GetSphere) (Variables|Character|GetMesh) "Root" "KeepRelative" "KeepRelative" "KeepRelative" true)
  (Pawn|Components|CharacterMovement|SetMovementMode (Variables|Character|GetCharacterMovement) "MOVE_Flying" 0 :!label _label)
  (if _returnvalue_2
    (bind _returnvalue_3 (Class|AnimMontage|CreateSlotAnimationasDynamicMontagewithBlendSettings _animsequence_to_test "Defaultslot" (Utilities|Struct|MakeMontageBlendSettings 0 _alphablendargs "Standard") (Utilities|Struct|MakeMontageBlendSettings 0 _alphablendargs "Standard") 1.0 1 -1.0)))
  (Animation|Montage|PlayMontage (Variables|Character|GetMesh) (select _returnvalue_2 _returnvalue_3 (Variables|Default|GetAnimation%20to%20test))
    (:OnCompleted
      (Pawn|Components|CharacterMovement|SetMovementMode (Variables|Character|GetCharacterMovement) "MOVE_Walking" 0)
      (Utilities|FlowControl|Delay 2.0)
      (Transformation|SetActorLocationAndRotation (Variables|Default|GetLocation) (Variables|Default|GetRot) false true)
      (goto _label))))